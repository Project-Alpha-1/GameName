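; Paper2D flipbook character, file name enmy, driven by player input to run, jump, dash and melee attack BP_Player actors.
; Enhanced Input handles movement, a velocity-polled jump landing and a dash that temporarily alters movement settings, while left click starts attacks.
; Tick fires a DoOnce hit check on attack frame 3, damaging Attackbox overlaps with blood effects.
; Incoming damage reduces Health and plays hit or death flipbooks, with animation completion restoring idle.
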(event `Key|LeftMouseButton`
  (params (Key :type "Key Structure"))
  (:`Pressed`
    (`PaperFlipbookComponent.SetFlipbook` (`self.Sprite`) "/Game/sheets/Blue/attck/Attck_B.Attck_B")
    (`PaperFlipbookComponent.SetLooping` (`self.Sprite`) false)
    (set `self.isAttacking` true)))

(event `self.Sprite.OnFinishedPlaying`
  (if (not (`self.isDead`))
    (`PaperFlipbookComponent.SetFlipbook` (`self.Sprite`) "/Game/sheets/Blue/idle/Idle_B.Idle_B")
    (`self.RestartAnim`)
    (set `self.isAttacking` false)
    (`self.Rest Attack`)
    (`SceneComponent.SetHiddenInGame` (`self.attackbox`) true false)))

(event `Rest Attack`
  (goto _label :!via `Reset`))

(event `self.ReceiveTick`
  (params (DeltaSeconds :type "Float (single-precision)"))
  (if (`self.isAttacking`)
    (if (== (`PaperFlipbookComponent.GetPlaybackPositionInFrames` (`self.Sprite`)) 3)
      (`/Engine/EditorBlueprintResources/StandardMacros.DoOnce` false :!label _label
        (:`Completed`
          (`self.hitCheck`)
          (`SceneComponent.SetHiddenInGame` (`self.attackbox`) true false)))
      (else
        (`SceneComponent.SetHiddenInGame` (`self.attackbox`) true false)))))

(event `self.ReceiveAnyDamage`
  (params (Damage :type "Float (single-precision)") (DamageType :type "DamageType Object Reference") (InstigatedBy :type "Controller Object Reference") (DamageCauser :type "Actor Object Reference"))
  (set `self.Health` (- (`self.Health`) Damage))
  (if (<= (`self.Health`) 0.0)
    (`PaperFlipbookComponent.SetFlipbook` (`self.Sprite`) "/Game/sheets/Blue/die/Die_B.Die_B")
    (`PaperFlipbookComponent.SetLooping` (`self.Sprite`) false)
    (set `self.isDead` true)
    (else
      (`PaperFlipbookComponent.SetFlipbook` (`self.Sprite`) "/Game/sheets/Blue/hit/Hit_B.Hit_B")
      (`PaperFlipbookComponent.SetLooping` (`self.Sprite`) false))))

(event `self.ReceiveBeginPlay`
  (bind _asbp_player_controller (cast `/Game/Blueprints/BP_PlayerController` (`self.GetController`)))
  (`EnhancedInputSubsystemInterface.AddMappingContext` (pcsubsystem `EnhancedInputLocalPlayerSubsystem` _asbp_player_controller) "/Game/Blueprints/IMC_Default.IMC_Default" 0 (struct)))

(event `EnhancedInput|/Game/Blueprints/Actions/IA_Movement`
  (params (ActionValue :type "Float (double-precision)") (ElapsedSeconds :type "Float (double-precision)") (TriggeredSeconds :type "Float (double-precision)") (InputAction :type "InputAction Object Reference" :default "/Game/Blueprints/Actions/IA_Movement.IA_Movement"))
  (:`Triggered`
    (if (not (`self.bIsJumping`))
      (`self.AddMovementInput` (`self.GetActorForwardVector`) ActionValue)
      (`PaperFlipbookComponent.SetFlipbook` (`self.Sprite`) "/Game/sheets/Blue/run/Run_B.Run_B")
      (if (> ActionValue 0.0)
        (`SceneComponent.K2_SetWorldRotation` :`self` (`self.Sprite`))
        (`SceneComponent.K2_AddLocalRotation` :`self` (`self.attackbox`))
        (else
          (`SceneComponent.K2_SetWorldRotation` (`self.Sprite`) (struct :`Yaw` -180.0) false false)
          (`SceneComponent.K2_AddLocalRotation` (`self.attackbox`) (struct :`Yaw` -180.0) false false)))))
  (:`Completed`
    (if (not (`self.bIsJumping`))
      (`PaperFlipbookComponent.SetFlipbook` (`self.Sprite`) "/Game/sheets/Blue/idle/Idle_B.Idle_B"))))

(event `EnhancedInput|/Game/Blueprints/Actions/IA_Jump`
  (params (ActionValue :type Boolean) (ElapsedSeconds :type "Float (double-precision)") (TriggeredSeconds :type "Float (double-precision)") (InputAction :type "InputAction Object Reference" :default "/Game/Blueprints/Actions/IA_Jump.IA_Jump"))
  (bind _sprite (`self.Sprite`))
  (:`Triggered`
    (if (not (`self.bIsJumping`))
      (set `self.bIsJumping` true)
      (`self.Jump`)
      (`PaperFlipbookComponent.SetLooping` _sprite false)
      (`PaperFlipbookComponent.SetFlipbook` _sprite "/Game/sheets/Blue/jump/Jump_B.Jump_B")
      (`KismetSystemLibrary.Delay` 0.1)
      (if (== (.z (`self.GetVelocity`)) 0.0) :!label _label_2
        (`PaperFlipbookComponent.SetLooping` _sprite true)
        (`PaperFlipbookComponent.Play` _sprite)
        (`PaperFlipbookComponent.SetFlipbook` _sprite "/Game/sheets/Blue/idle/Idle_B.Idle_B")
        (set `self.bIsJumping` false)
        (else
          (`KismetSystemLibrary.Delay` 0.1)
          (goto _label_2))))))

(event `EnhancedInput|/Game/Blueprints/Actions/IA_Dash`
  (params (ActionValue :type Boolean) (ElapsedSeconds :type "Float (double-precision)") (TriggeredSeconds :type "Float (double-precision)") (InputAction :type "InputAction Object Reference" :default "/Game/Blueprints/Actions/IA_Dash.IA_Dash"))
  (bind _charactermovement (`self.CharacterMovement`))
  (bind _charactermovement_2 (`self.CharacterMovement`))
  (:`Triggered`
    (if (not (`self.isDashing`))
      (set `self.isDashing` true)
      (set `CharacterMovementComponent.MaxWalkSpeed` 5000.0 _charactermovement_2)
      (`PaperFlipbookComponent.SetPlayRate` (`self.Sprite`) 5.0)
      (set `CharacterMovementComponent.MaxAcceleration` 5000.0 _charactermovement_2)
      (set `CharacterMovementComponent.BrakingFriction` 2000.0 _charactermovement_2)
      (`KismetSystemLibrary.K2_SetTimerDelegate` :`Time` 0.75)))
  (:`Completed`
    (set `CharacterMovementComponent.MaxWalkSpeed` 150.0 _charactermovement)
    (set `CharacterMovementComponent.MaxAcceleration` 2400.0 _charactermovement)
    (`KismetSystemLibrary.K2_SetTimerDelegate` (delegate `Reset Breaking Friction`) 0.2)))

(event `Reset Breaking Friction`
  (set `CharacterMovementComponent.BrakingFriction` 0.0 (`self.CharacterMovement`))
  (`PaperFlipbookComponent.SetPlayRate` (`self.Sprite`) 1.0)
  (set `self.isDashing` false))

(fn `hitCheck`
  (for _array_element (`PrimitiveComponent.GetOverlappingActors` (`self.attackbox`) "/Game/Blueprints/BP_Player.BP_Player_C")
    (if (!= _array_element self)
      (`GameplayStatics.ApplyDamage` _array_element (`self.Damage Amount`))
      (set `self.hitSomthing` true)))
  (if (`self.hitSomthing`)
    (`GameplayStatics.SpawnEmitterAtLocation` "/Game/Realistic_Starter_VFX_Pack_Vol2/Particles/Blood/P_Blood_Splat_Cone.P_Blood_Splat_Cone" (`SceneComponent.GetSocketLocation` (`self.Sprite`) "HitPos") (struct :`Pitch` -90.0) (0.5 0.3 0.2))
    (set `self.hitSomthing` false)))

(fn `RestartAnim`
  (`PaperFlipbookComponent.SetLooping` (`self.Sprite`) true)
  (if (not (`PaperFlipbookComponent.IsPlaying` (`self.Sprite`)))
    (`PaperFlipbookComponent.Play` (`self.Sprite`))))

(fn `UserConstructionScript`)