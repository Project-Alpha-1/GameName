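; Player-controlled Paper2D orc warrior character, despite its Enemy folder, with Enhanced Input for side-to-side walking, dashing and jumping.
; Each action swaps sprite flipbooks, and movement also rotates the sprite and axe capsule by direction.
; Dash boosts speed, acceleration and braking friction, with a delayed friction and animation reset after release.
; Jump blocks movement input and polls vertical velocity on a delay loop to detect landing.
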(event `self.ReceiveBeginPlay`
  (bind _asbp_player_controller (cast `/Game/Blueprints/BP_PlayerController` (`self.GetController`)))
  (`EnhancedInputSubsystemInterface.AddMappingContext` (pcsubsystem `EnhancedInputLocalPlayerSubsystem` _asbp_player_controller) "/Game/Blueprints/IMC_Default.IMC_Default" 0 (struct)))

(event `EnhancedInput|/Game/Blueprints/Actions/IA_Dash`
  (params (ActionValue :type Boolean) (ElapsedSeconds :type "Float (double-precision)") (TriggeredSeconds :type "Float (double-precision)") (InputAction :type "InputAction Object Reference" :default "/Game/Blueprints/Actions/IA_Dash.IA_Dash"))
  (bind _charactermovement (`self.CharacterMovement`))
  (bind _charactermovement_2 (`self.CharacterMovement`))
  ;[1 1 1] Sprint Movement
  (:`Triggered`
    (if (not (`self.isDashing`))
      (set `self.isDashing` true)
      (set `CharacterMovementComponent.MaxWalkSpeed` 5000.0 _charactermovement_2)
      (`PaperFlipbookComponent.SetFlipbook` (`self.Sprite`) "/Game/sheets/OrcWar/Flipbooks/OW_Run.OW_Run")
      (`PaperFlipbookComponent.SetPlayRate` (`self.Sprite`) 5.0)
      (set `CharacterMovementComponent.MaxAcceleration` 5000.0 _charactermovement_2)
      (set `CharacterMovementComponent.BrakingFriction` 2000.0 _charactermovement_2)
      (`KismetSystemLibrary.K2_SetTimerDelegate` :`Time` 0.75)))
  (:`Completed`
    (set `CharacterMovementComponent.MaxWalkSpeed` 150.0 _charactermovement)
    (set `CharacterMovementComponent.MaxAcceleration` 2400.0 _charactermovement)
    (`KismetSystemLibrary.K2_SetTimerDelegate` (delegate `Reset Breaking Friction`) 0.2)))

(event `Reset Breaking Friction`
  ;[1 1 1] Sprint Movement
  (set `CharacterMovementComponent.BrakingFriction` 0.0 (`self.CharacterMovement`))
  (`PaperFlipbookComponent.SetFlipbook` (`self.Sprite`) "/Game/sheets/OrcWar/Flipbooks/OW_Walk1.OW_Walk1")
  (`PaperFlipbookComponent.SetPlayRate` (`self.Sprite`) 1.0)
  (set `self.isDashing` false))

(event `EnhancedInput|/Game/Blueprints/Actions/IA_Jump`
  (params (ActionValue :type Boolean) (ElapsedSeconds :type "Float (double-precision)") (TriggeredSeconds :type "Float (double-precision)") (InputAction :type "InputAction Object Reference" :default "/Game/Blueprints/Actions/IA_Jump.IA_Jump"))
  (bind _sprite (`self.Sprite`))
  ;[1 1 1] Jump Movement
  (:`Triggered`
    (if (not (`self.isJumping`))
      (set `self.isJumping` true)
      (`self.Jump`)
      (`PaperFlipbookComponent.SetLooping` _sprite false)
      (`PaperFlipbookComponent.SetFlipbook` _sprite "/Game/sheets/OrcWar/Flipbooks/OW_Jump.OW_Jump")
      (`KismetSystemLibrary.Delay` 0.1)
      (if (== (.z (`self.GetVelocity`)) 0.0) :!label _label
        (`PaperFlipbookComponent.SetLooping` _sprite true)
        (`PaperFlipbookComponent.Play` _sprite)
        (`PaperFlipbookComponent.SetFlipbook` _sprite "/Game/sheets/OrcWar/Flipbooks/OW_Idle.OW_Idle")
        (set `self.isJumping` false)
        (else
          (`KismetSystemLibrary.Delay` 0.1)
          (goto _label))))))

(event `EnhancedInput|/Game/Blueprints/Actions/IA_Movement`
  (params (ActionValue :type "Float (double-precision)") (ElapsedSeconds :type "Float (double-precision)") (TriggeredSeconds :type "Float (double-precision)") (InputAction :type "InputAction Object Reference" :default "/Game/Blueprints/Actions/IA_Movement.IA_Movement"))
  ;[1 1 1] Movement
  (:`Triggered`
    (if (not (`self.isJumping`))
      (`self.AddMovementInput` (`self.GetActorForwardVector`) ActionValue)
      (`PaperFlipbookComponent.SetFlipbook` (`self.Sprite`) "/Game/sheets/OrcWar/Flipbooks/OW_Walk1.OW_Walk1")
      (if (> ActionValue 0.0)
        (`SceneComponent.K2_SetWorldRotation` :`self` (`self.Sprite`))
        (`SceneComponent.K2_AddLocalRotation` :`self` (`self.Axe_Capsule`))
        (else
          (`SceneComponent.K2_SetWorldRotation` (`self.Sprite`) (struct :`Yaw` -180.0) false false)
          (`SceneComponent.K2_AddLocalRotation` (`self.Axe_Capsule`) (struct :`Yaw` -180.0) false false)))))
  (:`Completed`
    (if (not (`self.isJumping`))
      (`PaperFlipbookComponent.SetFlipbook` (`self.Sprite`) "/Game/sheets/OrcWar/Flipbooks/OW_Idle.OW_Idle"))))

(event `self.ReceiveTick`
  (params (DeltaSeconds :type "Float (single-precision)")))

(fn `UserConstructionScript`)