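; EBP_OrcWar is a Paper2D orc enemy that walks along the X axis and reverses its facing when its capsule hits something.
; Each tick it picks a run or idle flipbook from velocity and sets sprite yaw from IsMovingRight, with movement input only toward -X when that flag is false.
; ChangeHealth adjusts and prints health; BeginPlay initializes it and adds an input mapping context if a BP_PlayerController possesses it.
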(event `self.ReceiveBeginPlay`
  (set `self.CurHealth` (`self.MaxHealth`))
  (bind _asbp_player_controller (cast `/Game/Blueprints/BP_PlayerController` (`self.GetController`)))
  (`EnhancedInputSubsystemInterface.AddMappingContext` (pcsubsystem `EnhancedInputLocalPlayerSubsystem` _asbp_player_controller) "/Game/Blueprints/IMC_Default.IMC_Default" 0 (struct)))

(event `AnimationUpdate`
  ;[1 1 1] Animation Update
  (`PaperFlipbookComponent.SetFlipbook` (`self.Sprite`) (select `bool` (> (`KismetMathLibrary.VSize` (`self.GetVelocity`)) 0.0) :`false` "/Game/sheets/OrcWar/Flipbooks/OW_Idle.OW_Idle" :`true` "/Game/sheets/OrcWar/Flipbooks/OW_Run.OW_Run" :!type "PaperFlipbook Object Reference")))

(event `Direction`
  ;[1 1 1] Direction Flip
  (`SceneComponent.K2_SetRelativeRotation` (`self.Sprite`) (`KismetMathLibrary.MakeRotator` 0.0 0.0 (`KismetMathLibrary.SelectFloat` 0.0 180.0 (`self.isMovingRight`))) false false)
  (`self.AddMovementInput` (`KismetMathLibrary.SelectVector` (0.0 0.0 0.0) (-1.0 0.0 0.0) (`self.isMovingRight`))))

(event `self.ReceiveTick`
  (params (DeltaSeconds :type "Float (single-precision)"))
  (`self.Direction`)
  (`self.AnimationUpdate`))

(event `self.CapsuleComponent.OnComponentHit`
  (params (HitComponent :type "PrimitiveComponent Object Reference") (OtherActor :type "Actor Object Reference") (OtherComp :type "PrimitiveComponent Object Reference") (NormalImpulse :type "Vector Structure") (Hit :type "HitResult Structure (by ref)"))
  (set `self.isMovingRight` (not (`self.isMovingRight`))))

(fn `ChangeHealth`
  (params (Amount :type "Float (double-precision)"))
  (bind _output_get (set `self.CurHealth` (+ (`self.CurHealth`) Amount)))
  (`KismetSystemLibrary.PrintString` (`KismetStringLibrary.Conv_DoubleToString` _output_get)))

(fn `UserConstructionScript`)